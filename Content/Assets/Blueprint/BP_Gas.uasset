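; BP_Gas is a grid-cell gas actor whose GasType sets its physical properties, material and Niagara color in Setup.
; A looping timer drives the simulation, using four 100-unit line traces along up, down, left and right.
; Spread spawns same-type copies into empty neighboring cells, then GasDensityPosition swaps positions with neighboring gases by comparing temperature/density/mass ratios.
; The older random-movement functions remain but are never run.
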(event Custom|Handle
  (CallFunction|Spread)
  (CallFunction|GasDensityPosition))

(event EventParticleData
  (params (Data :type Array%20of%20Basic%20Particle%20Data%20Structures) (NiagaraSystem :type Niagara%20System%20Object%20Reference) (SimulationPositionOffset :type Vector%20%28by%20ref%29 :default "0, 0, 0")))

(event EventBeginPlay
  (Class|NiagaraComponent|SetVariableObject (Variables|Default|GetGasEffect) "BPGAS" self)
  (CallFunction|Setup)
  (bind _returnvalue (Utilities|Time|SetTimerbyEvent (EventDispatchers|CreateEvent :!event Custom|Handle) (Variables|System|GetSpeedHandle) true))
  (Variables|Default|SetEvent_HandleMove _returnvalue))

(fn ConstructionScript
  (CallFunction|Setup))

(fn CheckPosOld
  (bind _returnvalue (Transformation|GetActorLocation))
  (bind _returnvalue_2 (Transformation|GetActorLocation))
  (bind _returnvalue_3 (Transformation|GetActorLocation))
  (bind _returnvalue_4 (Transformation|GetActorLocation))
  ;[1 1 1] Up
  (bind (_outhit _returnvalue_5) (Collision|LineTraceByChannel _returnvalue_4 (+ _returnvalue_4 (* (Math|Vector|GetUpVector (Transformation|GetActorRotation)) 100)) "TraceTypeQuery1" false 0 "Persistent"))
  (Utilities|Array|SetArrayElem (Variables|Default|GetLastHitDirection) 0 (select _returnvalue_5 _outhit (Collision|MakeHitResult false false 0.0 0.0 "0, 0, 0" "0, 0, 0" "0,0,1" "0,0,1" 0 0)))
  ;[1 1 1] Down
  (bind (_outhit_2 _returnvalue_6) (Collision|LineTraceByChannel _returnvalue_2 (+ _returnvalue_2 (* (Math|Vector|GetUpVector (Transformation|GetActorRotation)) -100)) "TraceTypeQuery1" false 0 "Persistent"))
  (Utilities|Array|SetArrayElem (Variables|Default|GetLastHitDirection) 1 (select _returnvalue_6 _outhit_2 (Collision|MakeHitResult false false 0.0 0.0 "0, 0, 0" "0, 0, 0" "0,0,1" "0,0,1" 0 0)))
  ;[1 1 1] Left
  (bind (_outhit_3 _returnvalue_7) (Collision|LineTraceByChannel _returnvalue_3 (+ _returnvalue_3 (* (Math|Vector|GetRightVector (Transformation|GetActorRotation)) -100)) "TraceTypeQuery1" false 0 "Persistent"))
  (Utilities|Array|SetArrayElem (Variables|Default|GetLastHitDirection) 2 (select _returnvalue_7 _outhit_3 (Collision|MakeHitResult false false 0.0 0.0 "0, 0, 0" "0, 0, 0" "0,0,1" "0,0,1" 0 0)))
  ;[1 1 1] Right
  (bind (_outhit_4 _returnvalue_8) (Collision|LineTraceByChannel _returnvalue (+ _returnvalue (* (Math|Vector|GetRightVector (Transformation|GetActorRotation)) 100)) "TraceTypeQuery1" false 0 "Persistent"))
  (Utilities|Array|SetArrayElem (Variables|Default|GetLastHitDirection) 2 (select _returnvalue_8 _outhit_4 (Collision|MakeHitResult false false 0.0 0.0 "0, 0, 0" "0, 0, 0" "0,0,1" "0,0,1" 0 0))))

(fn Setup
  (Variables|Info|SetTemperature (Utilities|Select :Index (Variables|Info|GetGasType) :NewEnumerator0 22.0 :NewEnumerator1 22.0 :NewEnumerator2 27.0 :NewEnumerator3 3e+01))
  (Variables|Info|SetDensity (Utilities|Select :Index (Variables|Info|GetGasType) :NewEnumerator0 15.9994 :NewEnumerator1 15.9995 :NewEnumerator2 44.01 :NewEnumerator3 1.00794))
  (Variables|Info|SetMass (Utilities|Select :Index (Variables|Info|GetGasType) :NewEnumerator0 1.8 :NewEnumerator1 1.8 :NewEnumerator2 1.8 :NewEnumerator3 1.8))
  (Variables|Info|SetIsBreathable (Utilities|Select :Index (Variables|Info|GetGasType) :NewEnumerator0 true :NewEnumerator1 false :NewEnumerator2 false :NewEnumerator3 false))
  (Variables|Info|SetSpecificHeatCapacity (Utilities|Select :Index (Variables|Info|GetGasType) :NewEnumerator0 1.005 :NewEnumerator1 1.01 :NewEnumerator2 0.846 :NewEnumerator3 2.4))
  (Variables|Info|SetThermalConductivity (Utilities|Select :Index (Variables|Info|GetGasType) :NewEnumerator0 0.024 :NewEnumerator1 0.024 :NewEnumerator2 0.015 :NewEnumerator3 0.168))
  (bind _cube (Variables|Default|GetCube)
    (:then
      (Rendering|Material|SetMaterial _cube 0 (Utilities|Select :Index (Variables|Info|GetGasType) :NewEnumerator0 "/Game/Assets/Materials/M_MasterColor_Oxygen.M_MasterColor_Oxygen" :NewEnumerator1 "/Game/Assets/Materials/M_MasterColor_OxygenPollued.M_MasterColor_OxygenPollued" :NewEnumerator2 "/Game/Assets/Materials/M_MasterColor_Dioxide.M_MasterColor_Dioxide" :NewEnumerator3 "/Game/Assets/Materials/M_MasterColor_Hydro.M_MasterColor_Hydro"))
      (bind _gaseffect (Variables|Default|GetGasEffect)
        (:then
          (Class|NiagaraComponent|SetNiagaraVariableVec4 _gaseffect "Color" (Utilities|Select :Index (Variables|Info|GetGasType) :NewEnumerator0 (Math|Vector4|MakeVector4 0.0 0.895053 1.0 1.0) :NewEnumerator1 (Math|Vector4|MakeVector4 0.0 1.0 0.275573 1.0) :NewEnumerator2 (Math|Vector4|MakeVector4 0.104167 0.104167 0.104167 1.0) :NewEnumerator3 (Math|Vector4|MakeVector4 1.0 0.0 0.669267 1.0))))
        (:else)))
    (:else)))

(fn CheckGasOld
  (for _array_element (Variables|Default|GetLastHitDirection)
    (Utilities|Array|Add (LocalVariables|GetCanMoveDirectional) (not (.bBlockingHit (Collision|BreakHitResult _array_element))))
    (Utilities|IsValid (.HitActor (Collision|BreakHitResult _array_element))
      (:Is%20Valid
        (LocalVariables|SetCanMove false)
        (bind _asbp_gas (Utilities|Casting|CastToBP_Gas (.HitActor (Collision|BreakHitResult _array_element))))
        (bind _output_get (LocalVariables|SetLocalLastHitBP _asbp_gas))
        (LocalVariables|SetLocalGasHit (Variables|BP_Gas_C|GetGasType _output_get))
        (if (!= (Variables|BP_Gas_C|GetDensity (LocalVariables|GetLocalLastHitBP)) 0.0)
          _))))
  (return (LocalVariables|GetCanMove) (LocalVariables|GetCanMoveDirectional)))

(fn MoveGasOld
  (params (MoveOutPut :type Array%20of%20Booleans))
  (bind _returnvalue (Transformation|GetActorLocation))
  (bind _returnvalue_2 (Transformation|GetActorLocation))
  (bind _returnvalue_3 (Transformation|GetActorLocation))
  (bind _returnvalue_4 (Transformation|GetActorLocation))
  (while (not (LocalVariables|GetLocalIsGood))
    (LocalVariables|SetLocalDirection (Math|Random|RandomInteger (- (Utilities|Array|Length MoveOutPut) 1)))
    (bind _output_get (LocalVariables|SetLocalSelectedMovePoint (Utilities|Array|Get(acopy) MoveOutPut (LocalVariables|GetLocalDirection))))
    (if _output_get
      ;[1 1 1] 0 = UP | 1 = DOWN | 2 = LEFT | 3 = RIGHT
      (switch int (LocalVariables|GetLocalDirection)
        (:0
          (Transformation|SetActorLocation (Math|Vector|MakeVector (.x _returnvalue_3) (.y _returnvalue_3) (+ (.z _returnvalue_3) 1e+02)) true false))
        (:1
          (Transformation|SetActorLocation (Math|Vector|MakeVector (.x _returnvalue_4) (.y _returnvalue_4) (- (.z _returnvalue_4) 1e+02)) true false))
        (:2
          (Transformation|SetActorLocation (Math|Vector|MakeVector (.x _returnvalue_2) (- (.y _returnvalue_2) 1e+02) (.z _returnvalue_2)) true false))
        (:3
          (Transformation|SetActorLocation (Math|Vector|MakeVector (.x _returnvalue) (+ (.y _returnvalue) 1e+02) (.z _returnvalue)) true false)))
      (LocalVariables|SetLocalIsGood true)
      (else
        (LocalVariables|SetLocalIsGood true)))))

(fn GasDensityPosition
  (bind _returnvalue (Transformation|GetActorLocation))
  (bind _returnvalue_2 (Transformation|GetActorLocation))
  (bind _returnvalue_3 (Transformation|GetActorLocation))
  (bind _returnvalue_4 (Transformation|GetActorLocation))
  (Utilities|FlowControl|Sequence
    (:then_0
      ;[1 1 1] Up
      (bind (_outhit _returnvalue_5) (Collision|LineTraceByChannel _returnvalue_4 (+ _returnvalue_4 (* (Math|Vector|GetUpVector (Transformation|GetActorRotation)) 100)) "TraceTypeQuery1" false 0 "None"))
      (if _returnvalue_5
        (bind _asbp_gas (Utilities|Casting|CastToBP_Gas (.HitActor (Collision|BreakHitResult _outhit))))
        (if (> (Utilities|Operators|Divide (Variables|Info|GetTemperature) (Variables|Info|GetDensity) (Variables|Info|GetMass)) (Utilities|Operators|Divide (Variables|BP_Gas_C|GetTemperature _asbp_gas) (Variables|BP_Gas_C|GetDensity _asbp_gas) (Variables|BP_Gas_C|GetMass _asbp_gas)))
          (bind _output_get (LocalVariables|SetLastLoc (Transformation|GetActorLocation _asbp_gas)))
          (Transformation|SetActorLocation _asbp_gas (Transformation|GetActorLocation) false false)
          (Transformation|SetActorLocation _output_get false false))))
    (:then_1
      ;[1 1 1] Down
      (bind (_outhit_2 _returnvalue_6) (Collision|LineTraceByChannel _returnvalue_2 (+ _returnvalue_2 (* (Math|Vector|GetUpVector (Transformation|GetActorRotation)) -100)) "TraceTypeQuery1" false 0 "None"))
      (if _returnvalue_6
        (bind _asbp_gas_2 (Utilities|Casting|CastToBP_Gas (.HitActor (Collision|BreakHitResult _outhit_2))))
        (if (> (Utilities|Operators|Divide (Variables|BP_Gas_C|GetTemperature _asbp_gas_2) (Variables|BP_Gas_C|GetDensity _asbp_gas_2) (Variables|BP_Gas_C|GetMass _asbp_gas_2)) (Utilities|Operators|Divide (Variables|Info|GetTemperature) (Variables|Info|GetDensity) (Variables|Info|GetMass)))
          (bind _output_get_2 (LocalVariables|SetLastLoc (Transformation|GetActorLocation)))
          (Transformation|SetActorLocation (Transformation|GetActorLocation _asbp_gas_2) false false)
          (Transformation|SetActorLocation _asbp_gas_2 _output_get_2 false false))))
    (:then_2
      ;[1 1 1] Left
      (bind (_outhit_3 _returnvalue_7) (Collision|LineTraceByChannel _returnvalue_3 (+ _returnvalue_3 (* (Math|Vector|GetRightVector (Transformation|GetActorRotation)) -100)) "TraceTypeQuery1" false 0 "None"))
      (if _returnvalue_7
        (bind _asbp_gas_3 (Utilities|Casting|CastToBP_Gas (.HitActor (Collision|BreakHitResult _outhit_3))))
        (if (> (Utilities|Operators|Divide (Variables|BP_Gas_C|GetTemperature _asbp_gas_3) (Variables|BP_Gas_C|GetDensity _asbp_gas_3) (Variables|BP_Gas_C|GetMass _asbp_gas_3)) (Utilities|Operators|Divide (Variables|Info|GetTemperature) (Variables|Info|GetDensity) (Variables|Info|GetMass)))
          (bind _output_get_3 (LocalVariables|SetLastLoc (Transformation|GetActorLocation)))
          (Transformation|SetActorLocation (Transformation|GetActorLocation _asbp_gas_3) false false)
          (Transformation|SetActorLocation _asbp_gas_3 _output_get_3 false false))))
    (:then_3
      ;[1 1 1] Right
      (bind (_outhit_4 _returnvalue_8) (Collision|LineTraceByChannel _returnvalue (+ _returnvalue (* (Math|Vector|GetRightVector (Transformation|GetActorRotation)) 100)) "TraceTypeQuery1" false 0 "None"))
      (if _returnvalue_8
        (bind _asbp_gas_4 (Utilities|Casting|CastToBP_Gas (.HitActor (Collision|BreakHitResult _outhit_4))))
        (if (> (Utilities|Operators|Divide (Variables|BP_Gas_C|GetTemperature _asbp_gas_4) (Variables|BP_Gas_C|GetDensity _asbp_gas_4) (Variables|BP_Gas_C|GetMass _asbp_gas_4)) (Utilities|Operators|Divide (Variables|Info|GetTemperature) (Variables|Info|GetDensity) (Variables|Info|GetMass)))
          (bind _output_get_4 (LocalVariables|SetLastLoc (Transformation|GetActorLocation)))
          (Transformation|SetActorLocation (Transformation|GetActorLocation _asbp_gas_4) false false)
          (Transformation|SetActorLocation _asbp_gas_4 _output_get_4 false false))))))

(fn Spread
  (bind _returnvalue (Transformation|GetActorLocation))
  (bind _returnvalue_2 (Transformation|GetActorLocation))
  (bind _returnvalue_3 (Transformation|GetActorLocation))
  (bind _returnvalue_4 (Transformation|GetActorLocation))
  (bind _returnvalue_5 (Transformation|GetActorLocation))
  (bind _returnvalue_6 (Transformation|GetActorLocation))
  (bind _returnvalue_7 (Transformation|GetActorLocation))
  (bind _returnvalue_8 (Transformation|GetActorLocation))
  (Utilities|FlowControl|Sequence
    (:then_0
      ;[1 1 1] Left
      (bind _returnvalue_9 (Collision|LineTraceByChannel _returnvalue_3 (+ _returnvalue_3 (* (Math|Vector|GetRightVector (Transformation|GetActorRotation)) -100)) "TraceTypeQuery1" false 0 "None"))
      (if (not _returnvalue_9)
        (Game|SpawnActorfromClass "BP_Gas_C" (Math|Transform|MakeTransform (Math|Vector|MakeVector (.x _returnvalue_5) (- (.y _returnvalue_5) 1e+02) (.z _returnvalue_5)) "0, 0, 0" "1.000000,1.000000,1.000000") "AlwaysSpawn" "MultiplyWithRoot" 0 (Variables|Info|GetGasType) 0)))
    (:then_1
      ;[1 1 1] Right
      (bind _returnvalue_10 (Collision|LineTraceByChannel _returnvalue (+ _returnvalue (* (Math|Vector|GetRightVector (Transformation|GetActorRotation)) 100)) "TraceTypeQuery1" false 0 "None"))
      (if (not _returnvalue_10)
        (Game|SpawnActorfromClass "BP_Gas_C" (Math|Transform|MakeTransform (Math|Vector|MakeVector (.x _returnvalue_6) (+ (.y _returnvalue_6) 1e+02) (.z _returnvalue_6)) "0, 0, 0" "1.000000,1.000000,1.000000") "AlwaysSpawn" "MultiplyWithRoot" 0 (Variables|Info|GetGasType) 0)))
    (:then_2
      ;[1 1 1] Up
      (bind _returnvalue_11 (Collision|LineTraceByChannel _returnvalue_8 (+ _returnvalue_8 (* (Math|Vector|GetUpVector (Transformation|GetActorRotation)) 100)) "TraceTypeQuery1" false 0 "None"))
      (if (not _returnvalue_11)
        (Game|SpawnActorfromClass "BP_Gas_C" (Math|Transform|MakeTransform (Math|Vector|MakeVector (.x _returnvalue_7) (.y _returnvalue_7) (+ (.z _returnvalue_7) 1e+02)) "0, 0, 0" "1.000000,1.000000,1.000000") "AlwaysSpawn" "MultiplyWithRoot" 0 (Variables|Info|GetGasType) 0)))
    (:then_3
      ;[1 1 1] Down
      (bind _returnvalue_12 (Collision|LineTraceByChannel _returnvalue_2 (+ _returnvalue_2 (* (Math|Vector|GetUpVector (Transformation|GetActorRotation)) -100)) "TraceTypeQuery1" false 0 "None"))
      (if (not _returnvalue_12)
        (Game|SpawnActorfromClass "BP_Gas_C" (Math|Transform|MakeTransform (Math|Vector|MakeVector (.x _returnvalue_4) (.y _returnvalue_4) (- (.z _returnvalue_4) 1e+02)) "0, 0, 0" "1.000000,1.000000,1.000000") "AlwaysSpawn" "MultiplyWithRoot" 0 (Variables|Info|GetGasType) 0)))))